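; BP_FloorManager feeds the position and size of a referenced Tree actor's static meshes into a referenced floor's material.
; Its construction script creates a dynamic material instance on FloorRef's first material slot.
; It then loops over the Tree's static mesh components, writing each world location and bounds radius to SphereLocation and Radius.
; Each pass overwrites the same two parameters, so only the last component's sphere remains.
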(fn `UserConstructionScript`
  (bind _staticmeshcomponent (`StaticMeshActor.StaticMeshComponent` (`self.FloorRef`)))
  (bind _returnvalue (`PrimitiveComponent.CreateDynamicMaterialInstance` _staticmeshcomponent 0 (`PrimitiveComponent.GetMaterial` _staticmeshcomponent 0) "None"))
  (for _array_element (`self.K2_GetComponentsByClass` (`self.Tree`) "/Script/Engine.StaticMeshComponent")
    (`MaterialInstanceDynamic.SetVectorParameterValue` _returnvalue "SphereLocation" (`KismetMathLibrary.Conv_VectorToLinearColor` (`SceneComponent.K2_GetComponentLocation` _array_element)))
    (`MaterialInstanceDynamic.SetScalarParameterValue` _returnvalue "Radius" (`.SphereRadius` (`KismetSystemLibrary.GetComponentBounds` _array_element)))))