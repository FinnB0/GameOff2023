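; BP_Tower is a tower actor that attacks on a repeating timer and can be destroyed.
; The construction script copies values from CombatStats into HealthComponent's max health and AttackComponent's animation duration.
; On BeginPlay a looping timer, paced by the attack speed stat, sends the attack type to AttackComponent.
; The actor destroys itself when HealthComponent signals zero health.
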(event `self.ReceiveBeginPlay`
  (`KismetSystemLibrary.K2_SetTimerDelegate` (delegate `Attack`) (`.AttackSpeed_10_E340079E4CB9068D7F684A97BC41BD8C` (break `/Game/Blueprints/CombatStats` (`self.CombatStats`))) true))

(event `Attack`
  (message `/Game/Blueprints/Interfaces/BPI_Attack.Attack` (`self.AttackComponent`) (`.AttackType_11_4C2107E842BB47F861168EBB7BAA4957` (break `/Game/Blueprints/CombatStats` (`self.CombatStats`)))))

(event `self.HealthComponent.Zero Health`
  (`self.K2_DestroyActor`))

(fn `UserConstructionScript`
  (set `/Game/Blueprints/Components/HealthComponent.Max Health` (`.Health_2_45B37E16496E77CB4791928E06522DCA` (break `/Game/Blueprints/CombatStats` (`self.CombatStats`))) (`self.HealthComponent`))
  (set `/Game/Blueprints/Components/AttackComponent.Animation Duration` (`.AttackSpeed_10_E340079E4CB9068D7F684A97BC41BD8C` (break `/Game/Blueprints/CombatStats` (`self.CombatStats`))) (`self.AttackComponent`)))