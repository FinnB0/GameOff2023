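; Game mode that runs the wave loop, switching play state between Paused, Building and Combat, and creates the HUD.
; Each wave fills an enemy list from DT_Waves and DT_NPCs, then a looping timer sends random entries to a spawn dispatcher.
; When the enemy count reaches zero, a Building countdown starts the next wave.
; It also fires music and sound triggers, and a tick gate slowly rotates the player view while Paused.
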(event `self.ReceiveBeginPlay`
  (bind _returnvalue (`GameplayStatics.GetPlayerController` 0))
  ;[1 1 1] EventBeginPlay
  (set `self.GameState_ref` (cast `/Game/Blueprints/Game/GSB_Game` (`GameplayStatics.GetGameState`) :!pure true))
  (`WidgetBlueprintLibrary.SetInputMode_GameAndUIEx` _returnvalue null)
  (set `PlayerController.bShowMouseCursor` true _returnvalue)
  (`AudioParameterControllerInterface.SetTriggerParameter` (`self.MSS_GameMusicTracks`) "OnMenu")
  ;[1 1 1] UI
  (bind _returnvalue_2 (`|CreateWidget` "/Game/Widgets/W_HUD.W_HUD_C"))
  (bind _output_get (set `self.HUD_ref` _returnvalue_2))
  (`UserWidget.AddToViewport` _output_get 0)
  (`self.SwitchGameState` "NewEnumerator0")
  ;[1 1 1] Grow Once at the start
  (`self.GrowMainTreeDispatcher`))

(event `UpdateMusic`
  ;[1 1 1] UpdateMusic
)

(event `SwitchGameState`
  (params (PGameState :type "/Game/Blueprints/Enums/E_GameState Enum" :default "NewEnumerator0"))
  ;[1 1 1] SwitchOnGameState
  (`/Game/Blueprints/Game/GSB_Game.SetPlayState` (`self.GameState_ref`) PGameState)
  (`self.UpdateMusic`)
  (switch `/Game/Blueprints/Enums/E_GameState` PGameState
    (:`NewEnumerator0`
      (`self.Sound_StopAmbient`)
      (`KismetSystemLibrary.Delay` 0.2)
      (`self.Sound_StartAmbient`)
      (`self.OpenTickGate`))
    (:`NewEnumerator1`
      (`self.Sound_StopAmbient`)
      (`KismetSystemLibrary.Delay` 0.2)
      (`self.Sound_StartAmbient`)
      (`self.CloseTickGate`))
    (:`NewEnumerator2`
      (`self.Sound_StopAmbient`)
      (`self.CloseTickGate`))))

(event `RandomizeMetaSound`
  ;[1 1 1] Randomize MEta Stuff (Trolling)
)

(event `self.ReceiveTick`
  (params (DeltaSeconds :type "Float (single-precision)"))
  ;[1 1 1] EventTick
  (`/Engine/EditorBlueprintResources/StandardMacros.Gate` false :!label _label
    (:`Exit`
      (`/Game/Blueprints/Player/BP_Player.Rotate` (cast `/Game/Blueprints/Player/BP_Player` (`GameplayStatics.GetPlayerPawn` 0) :!pure true) -0.1 false))))

(event `OpenTickGate`
  ;[1 1 1] EventTick
  (goto _label :!via `Open`))

(event `CloseTickGate`
  ;[1 1 1] EventTick
  (goto _label :!via `Close`))

(event `Sound_OnRoundStart`
  ;[1 1 1] Game-Sounds
  (`AudioParameterControllerInterface.SetTriggerParameter` (`self.MSS_GameSounds`) "OnRoundStart")
  (`AudioParameterControllerInterface.SetTriggerParameter` (`self.MSS_GameMusicTracks`) "OnWaveMode"))

(event `Sound_AttackTrigger`
  ;[1 1 1] NPC-Sounds
  (`AudioParameterControllerInterface.SetTriggerParameter` (`self.MSS_NPCSounds`) "OnAttackTrigger"))

(event `Sound_StartWalking`
  ;[1 1 1] NPC-Sounds
)

(event `Sound_OnStartAttacking`
  ;[1 1 1] Tree-Sounds
  (`AudioParameterControllerInterface.SetTriggerParameter` (`self.MSS_TreeSounds`) "OnStartAttacking"))

(event `Sound_OnRoundFInish`
  ;[1 1 1] Game-Sounds
  (`AudioParameterControllerInterface.SetTriggerParameter` (`self.MSS_GameSounds`) "OnRoundFinish")
  (`AudioParameterControllerInterface.SetTriggerParameter` (`self.MSS_GameMusicTracks`) "OnBuildMode"))

(event `Sound_StopWalking`
  ;[1 1 1] NPC-Sounds
)

(event `Sound_OnTimeRunsLOw`
  ;[1 1 1] Game-Sounds
  (`AudioParameterControllerInterface.SetTriggerParameter` (`self.MSS_GameSounds`) "OnTimeRunsLow"))

(event `Sound_OnStopAttacking`
  ;[1 1 1] Tree-Sounds
  (`AudioParameterControllerInterface.SetTriggerParameter` (`self.MSS_TreeSounds`) "OnStopAttacking"))

(event `Sound_OnDeath`
  ;[1 1 1] NPC-Sounds
  (`/Engine/EditorBlueprintResources/StandardMacros.DoOnce` false :!label _label_2
    (:`Completed`
      (`AudioParameterControllerInterface.SetTriggerParameter` (`self.MSS_NPCSounds`) "OnDeath")
      (`KismetSystemLibrary.Delay` 1.0)
      (goto _label_2 :!via `Reset`))))

(event `Sound_StartAmbient`
  ;[1 1 1] Game-Sounds
  (`AudioParameterControllerInterface.SetTriggerParameter` (`self.MSS_GameSounds`) "StartAmbient"))

(event `Sound_StopAmbient`
  ;[1 1 1] Game-Sounds
  (`AudioParameterControllerInterface.SetTriggerParameter` (`self.MSS_GameSounds`) "StopAmbient"))

(event `/Game/Blueprints/Interfaces/BPI_GameEssentials.StartGame`
  ;[1 1 1] StartGame
  (`self.StartNextWave`))

(event `StartNextWave`
  ;[1 1 1] Start Wave
  (`KismetSystemLibrary.K2_PauseTimerHandle` (`self.WaveCountdownTimer`))
  (`self.GrowMainTreeDispatcher`)
  (`self.StartSpawnTimer`)
  (`self.Sound_OnRoundStart`)
  (`self.Sound_StartWalking`))

(event `StartSpawnTimer`
  ;[1 1 1] SpawnTimer
  (`self.SwitchGameState` "NewEnumerator2")
  (`KismetSystemLibrary.Delay` 2.0)
  (`self.IncreaseSpawnAreaDispatcher`)
  (`self.SetupWaveData`)
  (bind _returnvalue (`KismetSystemLibrary.K2_SetTimerDelegate` (`|CreateDelegate` :!event `SpawnEnemy`) 0.1 true))
  (set `self.SpawnTimer` _returnvalue))

(event `SpawnEnemy`
  (bind (_outitem _outindex) (`KismetArrayLibrary.Array_Random` (`self.WaveEnemies`)))
  ;[1 1 1] SpawnTimer
  (`self.SpawnEnemyDispatcher` _outitem)
  (`KismetArrayLibrary.Array_Remove` (`self.WaveEnemies`) _outindex)
  (if (== (`KismetArrayLibrary.Array_Length` (`self.WaveEnemies`)) 0)
    (`KismetSystemLibrary.K2_PauseTimerHandle` (`self.SpawnTimer`))))

(event `/Game/Blueprints/Interfaces/BPI_GameEssentials.ReduceEnemyCount`
  ;[1 1 1] Reduces CurrentEnemyCount
  (bind _result (`/Engine/EditorBlueprintResources/StandardMacros.DecrementInt` (`self.CurrentEnemies`))
    (:`  `
      (if (== _result 0)
        (`self.SwitchGameState` "NewEnumerator1")
        (`self.StartNextWaveTimer`)
        (`self.Sound_OnRoundFInish`)
        (`self.Sound_StopWalking`)))))

(event `StartNextWaveTimer`
  ;[1 1 1] StartNextWaveTimer
  (set `self.WaveCountdownTime` 60)
  (bind _returnvalue (`KismetSystemLibrary.K2_SetTimerDelegate` (`|CreateDelegate` :!event `WaveCountDownTick`) 1.0 true))
  (set `self.WaveCountdownTimer` _returnvalue))

(event `WaveCountDownTick`
  ;[1 1 1] StartNextWaveTimer
  (bind _result (`/Engine/EditorBlueprintResources/StandardMacros.DecrementInt` (`self.WaveCountdownTime`))
    (:`  `
      (if (== _result 0)
        (`self.StartNextWave`)
        (elif (== _result 5)
          (`self.Sound_OnTimeRunsLOw`))))))

(fn `GetCurrentEnemies`
  (returns (CurrentEnemies :type Integer))
  (return (`self.CurrentEnemies`)))

(fn `GetTotalEnemies`
  (returns (TotalEnemies :type Integer))
  (return (`self.TotalEnemies`)))

(fn `GetWaveCount`
  (returns (WaveCount :type Integer))
  (return (`self.WaveCount`)))

(fn `GetWaveCountdownTime`
  (returns (WaveCountdownTime :type Integer))
  (return (`self.WaveCountdownTime`)))

(fn `GetWaveCountdownTimeMax`
  (returns (WaveCountdownTimeMax :type Integer))
  (return (`self.WaveCountdownTimeMax`)))

(fn `SetupWaveData`
  ;[1 1 1] Increases WaveCount / Goes through DT_Waves and Adds the correct EnemyStruct for every Enemy into the WaveEnemies Array
  (`KismetArrayLibrary.Array_Clear` (`self.WaveEnemies`))
  (bind _result (`/Engine/EditorBlueprintResources/StandardMacros.IncrementInt` (`self.WaveCount`))
    (:`  `
      (bind _returnvalue (`|GetDataTableRow` "/Game/Blueprints/Structs_Tables/DT_Waves.DT_Waves" (`KismetStringLibrary.Conv_StringToName` (`KismetStringLibrary.Conv_IntToString` _result)))
        (:`then`
          (bind ((`Enemy_Types_10_13560A524952CCEBF846A3B40835A471` _enemy_types) (`Enemy_Amount_6_C2AABAB2422B490A2AA963B99F9E3F10` _enemy_amount)) (break `/Game/Blueprints/Structs_Tables/ST_Waves` _returnvalue))
          (for (_array_element _array_index) _enemy_amount
            (for _ (range 1 (+ _array_element 1))
              (bind _returnvalue_2 (`|GetDataTableRow` "/Game/Blueprints/Structs_Tables/DT_NPCs.DT_NPCs" (`KismetStringLibrary.Conv_StringToName` (`|GetEnumeratorNameAsString` (`|GetArrayItem` _enemy_types _array_index))))
                (:`then`
                  (`KismetArrayLibrary.Array_Add` (`self.WaveEnemies`) _returnvalue_2)))))
          (bind _output_get (set `self.TotalEnemies` (`KismetArrayLibrary.Array_Length` (`self.WaveEnemies`))))
          (set `self.CurrentEnemies` _output_get))))))

(fn `UserConstructionScript`)