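; Tower actor that attacks pawns in range and can be selected or recycled for a refund of half its cost in seeds.
; Range-sphere overlaps toggle IsAttacking on the tree AnimBP, while Attack forwards to AttackComponent; the older looping-timer path is disconnected.
; Construction copies CombatStats into the component and sphere, scaling range and damage with wave count.
; BeginPlay binds to the GameMode's GrowMainTree dispatcher.
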(event `self.ReceiveBeginPlay`
  (`self.GetGM`))

(event `self.AttackRangeCollider.OnComponentBeginOverlap`
  (params (OverlappedComponent :type "PrimitiveComponent Object Reference") (OtherActor :type "Actor Object Reference") (OtherComp :type "PrimitiveComponent Object Reference") (OtherBodyIndex :type Integer) (bFromSweep :type Boolean) (SweepResult :type "HitResult Structure (by ref)"))
  ;[1 1 1] OnBeginOverlap AttackRangeCollider start AttackTimer
  (`self.SetAttacking` true))

(event `/Game/Blueprints/Interfaces/BPI_Interact.Recycle`
  ;[1 1 1 1 30] Interactions
  ;;[1 1 1] Recycles Tower (Stops overlapping and attacking instantly / Give Player 50% of Costs back / Destroy Tower)
  (set `PrimitiveComponent.bGenerateOverlapEvents` false (`self.AttackRangeCollider`))
  (`KismetSystemLibrary.K2_PauseTimerHandle` (`self.AttackTimer`))
  (message `/Game/Blueprints/Interfaces/BPI_Bounty.AddSeeds` (`GameplayStatics.GetPlayerPawn` 0) (/ (`self.Costs`) 2))
  (`self.K2_DestroyActor`))

(event `/Game/Blueprints/Interfaces/BPI_Interact.Select`
  ;[1 1 1 1 30] Interactions
  ;;[1 1 1] Selects Tower
  (`KismetSystemLibrary.PrintString` (`KismetStringLibrary.Concat_StrStr` (`KismetSystemLibrary.GetDisplayName` self) " is Selected!")))

(event `self.AttackRangeCollider.OnComponentEndOverlap`
  (params (OverlappedComponent :type "PrimitiveComponent Object Reference") (OtherActor :type "Actor Object Reference") (OtherComp :type "PrimitiveComponent Object Reference") (OtherBodyIndex :type Integer))
  ;[1 1 1] OnEndOverlap AttackRangeCollider stop AttackTimer IF there are no more Pawns nearby
  (if (== (`KismetArrayLibrary.Array_Length` (`PrimitiveComponent.GetOverlappingActors` (`self.AttackRangeCollider`) "/Script/Engine.Pawn")) 0)
    (`self.SetAttacking` false)))

(event `/Game/Blueprints/Interfaces/BPI_Attack.Attack`
  (params (`Attack Type` :type "/Game/Blueprints/Components/AttackTypes Enum" :default "NewEnumerator0"))
  ;[1 1 1] Attack
  (message `/Game/Blueprints/Interfaces/BPI_Attack.Attack` (`self.AttackComponent`) (`.AttackType_16_4C2107E842BB47F861168EBB7BAA4957` (break `/Game/Blueprints/Tower/CombatStats` (`self.CombatStats`)))))

(fn `GetGM`
  (bind _asgmb_game (cast `/Game/Blueprints/Game/GMB_Game` (`GameplayStatics.GetGameMode`)))
  (add `/Game/Blueprints/Game/GMB_Game.GrowMainTreeDispatcher` _asgmb_game (`|CreateDelegate` :!event `SetStats`)))

(fn `SetAttacking`
  (params (bIsAttacking :type Boolean))
  (bind _asab_maintree (cast `/Game/Meshes/Tree/Animations/AB_Maintree` (`SkeletalMeshComponent.GetAnimInstance` (`self.TowerSkeletalMesh`))))
  (set `/Game/Meshes/Tree/Animations/AB_Maintree.bIsAttacking` bIsAttacking _asab_maintree))

(fn `SetStats`
  (bind _attackcomponent (`self.AttackComponent`))
  (bind ((`Damage_4_B5A3B6D048C85AF64BF085A021E7EE73` _damage) (`AttackSpeed_15_E340079E4CB9068D7F684A97BC41BD8C` _attackspeed) (`AttackRange_17_186D62CB44D71BF6680F1280B938F158` _attackrange)) (break `/Game/Blueprints/Tower/CombatStats` (`self.CombatStats`)))
  ;[1 1 1] Set the relevant Stats in the component
  (bind _wavecount (message `/Game/Blueprints/Interfaces/BPI_GameEssentials.GetWaveCount` (`GameplayStatics.GetGameMode`)))
  (set `/Game/Blueprints/Components/AttackComponent.Animation Duration` _attackspeed _attackcomponent)
  (bind _returnvalue (+ (* (`KismetMathLibrary.Clamp` _wavecount 0 10000) 0.1) 1.0))
  (bind _returnvalue_2 (* _attackrange _returnvalue))
  (set `/Game/Blueprints/Components/AttackComponent.Range` _returnvalue_2 _attackcomponent)
  (set `/Game/Blueprints/Components/AttackComponent.Damage` (* _damage _returnvalue) _attackcomponent)
  ;[1 1 1] Use AttackRange from CombatStats for AttackRangeCollider
  (`SphereComponent.SetSphereRadius` (`self.AttackRangeCollider`) _returnvalue_2 true))

(fn `UserConstructionScript`
  (`self.SetStats`))