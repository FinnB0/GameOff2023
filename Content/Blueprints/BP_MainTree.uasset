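; Tree actor that repeatedly grows on a short timed loop, smoothly scaling up via a timeline while spreading procedural roots.
; RootGrowth first rings the trunk with ground-traced root meshes, then promotes roots to second-generation meshes and extends older ones with randomly rotated, possibly split tips.
; Forward traces destroy world-static actors in the roots' path, and new extensions are inverse-scaled to offset the growing tree.
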(event `self.ReceiveBeginPlay`
  (`KismetSystemLibrary.Delay` 2.0 :!label _label)
  (`self.Grow`)
  (goto _label))

(event `Grow`
  (bind _actorscaletemp (`self.ActorScaleTemp`))
  ;[0.07292 0.07292 0.07292] Growing
  ;;[1 1 1] Grows the roots
  ;; around the Tree
  (`self.RootGrowth`)
  ;;[1 1 1] Allows a smooth grow animation
  (set `self.ActorScaleTemp` (`self.GetActorScale3D`))
  (bind (_direction _scaletrack) (`Timeline|SmoothGrowTimer` :!via `PlayFromStart`)
    (:`Update`
      (`self.SetActorScale3D` (`KismetMathLibrary.VLerp` _actorscaletemp (+ _actorscaletemp (`self.GrowFactor`)) _scaletrack)))))

(fn `RandomRootRotation`
  (params (ParentRootRotation :type "Rotator Structure"))
  (returns (NextRootRotation :type "Rotator Structure"))
  (bind _rootgrowdirection (`self.RootGrowDirection`))
  (return (`KismetMathLibrary.MakeRotator` 0.0 0.0 (+ (.yaw ParentRootRotation) (`KismetMathLibrary.RandomFloatInRange` (* _rootgrowdirection -0.99) _rootgrowdirection)))))

(fn `RootGrowth`
  (bind _firstrootamount (`self.FirstRootAmount`))
  (bind _firstrootradiuslocationshift (`self.FirstRootRadiusLocationShift`))
  (bind _temporaryroots (`self.TemporaryRoots`))
  (`/Engine/EditorBlueprintResources/StandardMacros.IncrementInt` (`self.Iteration`)
    (:`  `
      (if (`self.bIsFirstGrowth`)
        (set `self.bIsFirstGrowth` false)
        ;[1 1 1] Creating the first FirstGenRoots around the Tree
        (for _index (range 1 (+ _firstrootamount 1))
          (bind _returnvalue (+ (`self.K2_GetActorLocation`) (* (`KismetMathLibrary.GetForwardVector` (`KismetMathLibrary.MakeRotator` 0.0 0.0 (+ (`KismetMathLibrary.Conv_IntToDouble` (* _index (/ 360 _firstrootamount))) (`KismetMathLibrary.RandomFloatInRange` (* _firstrootradiuslocationshift -1.0) _firstrootradiuslocationshift)))) (`KismetMathLibrary.RandomFloatInRange` 450.0 500.0)) (0.0 0.0 100.0)))
          (bind _outhit (`KismetSystemLibrary.LineTraceSingleForObjects` _returnvalue (- _returnvalue (0.0 0.0 200.0)) (`|MakeArray` "ObjectTypeQuery1" :!type "EObjectTypeQuery Enum")))
          (bind (_bblockinghit _binitialoverlap _time _distance _location _impactpoint) (`GameplayStatics.BreakHitResult` _outhit))
          (if _bblockinghit
            (bind _returnvalue_2 (`AddComponent|NODE_AddStaticMeshComponent-0` :`RelativeTransform` (`KismetMathLibrary.MakeTransform` _impactpoint (`KismetMathLibrary.MakeRotFromX` (- _impactpoint (`self.K2_GetActorLocation`))))))
            (`StaticMeshComponent.SetStaticMesh` _returnvalue_2 (`KismetArrayLibrary.Array_Random` (`self.FirstRootMeshCollection`)))
            (`KismetArrayLibrary.Array_Add` (`self.FirstGenRoots`) _returnvalue_2)))
        (else
          ;[1 1 1] Make every FirstGenRoot a TemporaryRoot
          (bind (_arrayindex _arrayelement) (`/Engine/EditorBlueprintResources/StandardMacros.ReverseForEachLoop` (`self.FirstGenRoots`))
            (:`LoopBody`
              (bind _returnvalue_3 (+ (.location (`SceneComponent.K2_GetComponentToWorld` _arrayelement)) (0.0 0.0 100.0)))
              (bind _outhit_2 (`KismetSystemLibrary.LineTraceSingleForObjects` _returnvalue_3 (+ _returnvalue_3 (* (`KismetMathLibrary.GetForwardVector` (.rotation (`SceneComponent.K2_GetComponentToWorld` _arrayelement))) (`KismetMathLibrary.RandomFloatInRange` (`self.MinRootGrowDistance`) (`self.MaxRootGrowDistance`)))) (`|MakeArray` "ObjectTypeQuery1" :!type "EObjectTypeQuery Enum")))
              (bind (_bblockinghit_2 _binitialoverlap_2 _time_2 _distance_2 _location_2 _impactpoint_2 _normal _impactnormal _physmat _hitactor) (`GameplayStatics.BreakHitResult` _outhit_2))
              (if _bblockinghit_2
                (`self.K2_DestroyActor` _hitactor))
              (`StaticMeshComponent.SetStaticMesh` _arrayelement (`KismetArrayLibrary.Array_Random` (`self.SecondRootMeshCollection`)))
              (`KismetArrayLibrary.Array_Add` (`self.TemporaryRoots`) _arrayelement)
              (`KismetArrayLibrary.Array_Remove` (`self.FirstGenRoots`) _arrayindex))
            (:`Completed`
              ;[1 1 1] For every SecondGenRoot Add a FirstGenRoot infront of it (with a possibilty of splitting)
              (bind (_arrayindex_2 _arrayelement_2) (`/Engine/EditorBlueprintResources/StandardMacros.ReverseForEachLoop` (`self.SecondGenRoots`))
                (:`LoopBody`
                  (bind _rotation (.rotation (`SceneComponent.K2_GetComponentToWorld` _arrayelement_2)))
                  (bind _returnvalue_4 (+ (.location (`SceneComponent.K2_GetComponentToWorld` _arrayelement_2)) (0.0 0.0 100.0)))
                  (bind _outhit_3 (`KismetSystemLibrary.LineTraceSingleForObjects` _returnvalue_4 (+ _returnvalue_4 (* (`KismetMathLibrary.GetForwardVector` _rotation) (`KismetMathLibrary.RandomFloatInRange` (`self.MinRootGrowDistance`) (`self.MaxRootGrowDistance`)) (.x (.scale (`SceneComponent.K2_GetComponentToWorld` _arrayelement_2))))) (`|MakeArray` "ObjectTypeQuery1" :!type "EObjectTypeQuery Enum")))
                  (bind (_bblockinghit_3 _binitialoverlap_3 _time_3 _distance_3 _location_3 _impactpoint_3 _normal_2 _impactnormal_2 _physmat_2 _hitactor_2 _hitcomponent _hitbonename _bonename _hititem _elementindex _faceindex _tracestart _traceend) (`GameplayStatics.BreakHitResult` _outhit_3))
                  (if _bblockinghit_3
                    (`self.K2_DestroyActor` _hitactor_2))
                  (bind _outhit_4 (`KismetSystemLibrary.LineTraceSingleForObjects` _traceend (- _traceend (0.0 0.0 200.0)) (`|MakeArray` "ObjectTypeQuery1" :!type "EObjectTypeQuery Enum")))
                  (bind (_bblockinghit_4 _binitialoverlap_4 _time_4 _distance_4 _location_4 _impactpoint_4) (`GameplayStatics.BreakHitResult` _outhit_4))
                  (if _bblockinghit_4
                    (for _index_2 (range (+ (`KismetMathLibrary.Conv_BoolToInt` (`KismetMathLibrary.RandomBoolWithWeight` (`self.RootSplitPossibility`))) 1))
                      (bind _returnvalue_5 (`AddComponent|NODE_AddStaticMeshComponent-16` :`RelativeTransform` (`KismetMathLibrary.MakeTransform` (`KismetMathLibrary.InverseTransformLocation` (`self.GetTransform`) (`KismetMathLibrary.SelectVector` (+ _impactpoint_4 (150.0 0.0 0.0)) _impactpoint_4 (== _index_2 1))) (`self.RandomRootRotation` _rotation) (`KismetMathLibrary.Conv_DoubleToVector` (/ 1.0 (.x (`self.GetActorScale3D`)))))))
                      (`StaticMeshComponent.SetStaticMesh` _returnvalue_5 (`KismetArrayLibrary.Array_Random` (`self.FirstRootMeshCollection`)))
                      (`KismetArrayLibrary.Array_Add` (`self.FirstGenRoots`) _returnvalue_5))
                    (`KismetArrayLibrary.Array_Remove` (`self.SecondGenRoots`) _arrayindex_2)))
                (:`Completed`
                  ;[1 1 1] Make every TemporaryRoot a SecondGenRoot
                  (set `self.SecondGenRoots` _temporaryroots)
                  (`KismetArrayLibrary.Array_Clear` _temporaryroots))))))))))

(fn `UserConstructionScript`)