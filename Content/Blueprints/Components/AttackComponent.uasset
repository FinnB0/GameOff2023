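; Attack component that lets its owning actor damage nearby actors tagged Enemy that implement BPI_Health.
; Attack branches on attack type: single-target uses one sphere trace, melee AoE a multi-sphere trace, and ranged AoE is unimplemented.
; For each target found, it fires OnAttack and uses a Delay of AnimationDuration before sending damage, with that Delay sitting inside the AoE loop.
; Both traces center on the owner with radius Range and draw debug shapes.
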(event `/Game/Blueprints/Interfaces/BPI_Attack.Attack`
  (params (`Attack Type` :type "/Game/Blueprints/Components/AttackTypes Enum" :default "NewEnumerator0"))
  ;[1 1 1] Pick a Calculation based on the Attack Type Enum
  ; The Delay should match the animation time
  (switch `/Game/Blueprints/Components/AttackTypes` `Attack Type`
    (:`NewEnumerator0`
      (bind _hitactor (`self.Find Target in Range`))
      (`self.On Attack`)
      (`KismetSystemLibrary.Delay` (`self.Animation Duration`))
      (message `/Game/Blueprints/Interfaces/BPI_Health.Apply Damage` _hitactor (`self.Damage`)))
    (:`NewEnumerator1`
      (bind _hitactor_2 (`self.Find Target in Melee Range`))
      (for _array_element _hitactor_2
        (`self.On Attack`)
        (`KismetSystemLibrary.Delay` (`self.Animation Duration`))
        (message `/Game/Blueprints/Interfaces/BPI_Health.Apply Damage` _array_element (`self.Damage`))))
    (:`NewEnumerator2`
      (`KismetSystemLibrary.PrintString` "Not implemented"))))

(fn `Find Target in Melee Range`
  (returns (HitActor :type "Array of Actor Object Reference"))
  (locals (`Hit Actor` :type "Array of Actor Object Reference"))
  (bind _returnvalue (`Actor.K2_GetActorLocation` (`self.GetOwner`)))
  ;[1 1 1] Use a Multisphere Trace to get all enemies in range
  (bind _outhits (`KismetSystemLibrary.SphereTraceMultiForObjects` :`Start` _returnvalue :`End` _returnvalue :`Radius` (`self.Range`) :`ObjectTypes` (`|MakeArray` "ObjectTypeQuery3" :!type "EObjectTypeQuery Enum") :`DrawDebugType` "ForDuration" :`DrawTime` 1.0))
  (for _array_element _outhits
    (bind (_bblockinghit _binitialoverlap _time _distance _location _impactpoint _normal _impactnormal _physmat _hitactor) (`GameplayStatics.BreakHitResult` _array_element))
    (if (and (`KismetSystemLibrary.DoesImplementInterface` _hitactor "/Game/Blueprints/Interfaces/BPI_Health.BPI_Health_C") (`Actor.ActorHasTag` _hitactor "Enemy"))
      (`KismetArrayLibrary.Array_Add` (`local.Hit Actor`) _hitactor)
      (else
        (`KismetSystemLibrary.PrintString` "False"))))
  (return (`local.Hit Actor`)))

(fn `Find Target in Range`
  (returns (HitActor :type "Actor Object Reference"))
  (bind _returnvalue (`Actor.K2_GetActorLocation` (`self.GetOwner`)))
  ;[1 1 1] Use a Sphere trace to find the closest enemy
  (bind _outhit (`KismetSystemLibrary.SphereTraceSingleForObjects` :`Start` _returnvalue :`End` _returnvalue :`Radius` (`self.Range`) :`ObjectTypes` (`|MakeArray` "ObjectTypeQuery3" :!type "EObjectTypeQuery Enum") :`DrawDebugType` "ForDuration" :`DrawTime` 1.0))
  (bind (_bblockinghit _binitialoverlap _time _distance _location _impactpoint _normal _impactnormal _physmat _hitactor) (`GameplayStatics.BreakHitResult` _outhit))
  (if (and (`KismetSystemLibrary.DoesImplementInterface` _hitactor "/Game/Blueprints/Interfaces/BPI_Health.BPI_Health_C") (`Actor.ActorHasTag` _hitactor "Enemy"))
    (return _hitactor)
    (else
      (`KismetSystemLibrary.PrintString` "False"))))