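; Health component that tracks current health for its owning actor and signals when it runs out.
; Health starts at MaxHealth on BeginPlay, and events apply damage, add healing without clamping to the maximum, or restore it fully.
; When damage brings health to zero or below, a DoOnce fires ZeroHealth a single time, with no reset even after healing.
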(event `self.ReceiveBeginPlay`
  (`self.Fully restore Health`))

(event `self.Apply Damage`
  (params (Damage :type Integer))
  (set `self.Current Health` (- (`self.Current Health`) Damage))
  (if (<= (`self.Current Health`) 0)
    (`/Engine/EditorBlueprintResources/StandardMacros.DoOnce` false
      (:`Completed`
        (`self.Zero Health`)))))

(event `self.Apply Heal`
  (params (`Health Points` :type Integer))
  (set `self.Current Health` (+ `Health Points` (`self.Current Health`))))

(event `self.Fully restore Health`
  (set `self.Current Health` (`self.Max Health`)))