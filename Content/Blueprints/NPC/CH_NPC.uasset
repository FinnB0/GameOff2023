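; Enemy NPC in a defense game that attacks the main tree and pays a seed bounty when killed.
; SetVariables configures stats, mesh, animation, strong-variant material and slightly randomized movement speed from a data struct.
; ApplyDamage subtracts armor with a minimum of one, then Kill awards seeds and spawns death VFX.
; Remove instead damages BP_MainTree; both exits reduce the GameMode's enemy count and destroy the actor.
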(event `self.ReceiveBeginPlay`)

(event `self.Apply Damage`
  (params (Damage :type Integer))
  (bind _returnvalue (- Damage (`self.Armor_Current`)))
  ;[1 1 1] Apply Damage (if HPCurrent==0 Player gets Bounty and Actor gets destroyed)
  (bind _output_get (set `self.HP_Current` (- (`self.HP_Current`) (`KismetMathLibrary.SelectInt` 1 _returnvalue (< _returnvalue 1)))))
  (if (<= _output_get 0)
    (`/Engine/EditorBlueprintResources/StandardMacros.DoOnce` false
      (:`Completed`
        (`/Game/Blueprints/Game/GMB_Game.Sound_OnDeath` (cast `/Game/Blueprints/Game/GMB_Game` (`GameplayStatics.GetGameMode`) :!pure true))
        (`self.Kill`)))))

(event `self.Kill`
  ;[1 1 1] InterfaceCall Kill / Adds Seeds to Player / RemoveEnemy in Spawner by RemoveEnemyDispatcher / Destroys Actor
  (message `/Game/Blueprints/Interfaces/BPI_Bounty.AddSeeds` (`GameplayStatics.GetPlayerPawn` 0) (`self.Bounty`))
  (message `/Game/Blueprints/Interfaces/BPI_GameEssentials.ReduceEnemyCount` (`GameplayStatics.GetGameMode`))
  (`NiagaraFunctionLibrary.SpawnSystemAtLocation` "/Game/FX/NS_EnemyDeath.NS_EnemyDeath" (`self.K2_GetActorLocation`) (struct) (`self.GetActorScale3D`))
  (`self.K2_DestroyActor`))

(event `self.Remove`
  ;[1 1 1] InterfaceCall Remove / Remove Enemy in Spawner by RemoveEnemyDispatcher / Destroys Actor
  (message `/Game/Blueprints/Interfaces/BPI_GameEssentials.ReduceEnemyCount` (`GameplayStatics.GetGameMode`))
  (bind _asc_npc (cast `/Game/Blueprints/NPC/C_NPC` (`AIBlueprintHelperLibrary.GetAIController` self)))
  ;;[1 0.5 0] no Backward logic -> no movement + resolve reference bug
  (`/Game/Blueprints/NPC/C_NPC.BT_Change_Walk_Direction` _asc_npc true)
  (`/Game/Blueprints/Game/GMB_Game.Sound_AttackTrigger` (cast `/Game/Blueprints/Game/GMB_Game` (`GameplayStatics.GetGameMode`) :!pure true))
  (bind _returnvalue (`GameplayStatics.GetActorOfClass` "/Game/Blueprints/BP_MainTree.BP_MainTree_C"))
  (message `/Game/Blueprints/Interfaces/BPI_Health.Apply Damage` (`/Game/Blueprints/BP_MainTree.HealthComponent` _returnvalue) (`self.Attack_Current`))
  (`self.K2_DestroyActor`))

(fn `Set_Variables`
  (params (ST_NPC :type "/Game/Blueprints/Structs_Tables/ST_NPCs Structure"))
  (bind (_st_npc_name _st_npc_description _st_npc_hp _st_npc_armor _st_npc_walkspeed _st_npc_attack _st_npc_bounty _st_npc_attacktype _st_npc_epoch _st_npc_mesh _st_npc_animclass _st_npc_m_strongversion) (break `/Game/Blueprints/Structs_Tables/ST_NPCs` (`self.ST_NPC`)))
  (set `self.ST_NPC` ST_NPC)
  (bind _output_get (set `self.HP_Max` _st_npc_hp))
  (set `self.HP_Current` _output_get)
  (bind _output_get_2 (set `self.Armor_Max` _st_npc_armor))
  (set `self.Armor_Current` _output_get_2)
  (bind _output_get_3 (set `self.WalkSpeed_Max` _st_npc_walkspeed))
  (set `self.WalkSpeed_Current` _output_get_3)
  (bind _output_get_4 (set `self.Attack_Max` _st_npc_attack))
  (set `self.Attack_Current` _output_get_4)
  (set `self.Bounty` _st_npc_bounty)
  (set `self.AttackType` _st_npc_attacktype)
  ;[1 1 1] Sets SkeletalMesh and AnimationBlueprint if SkeletalMeshfrom struct is Valid
  (`/Engine/EditorBlueprintResources/StandardMacros.IsValid` _st_npc_m_strongversion
    (:`Is Valid`
      (`PrimitiveComponent.SetMaterial` (`self.SK_Body`) 3 _st_npc_m_strongversion)
      (`PrimitiveComponent.SetMaterial` (`self.SK_Body`) 5 _st_npc_m_strongversion)
      (`/Engine/EditorBlueprintResources/StandardMacros.IsValid` _st_npc_mesh
        (:`Is Valid`
          _)
        (:`Is Not Valid`
          _)))
    (:`Is Not Valid`
      _))
  (`SkeletalMeshComponent.SetSkeletalMeshAsset` (`self.SK_Body`) _st_npc_mesh)
  (`SkeletalMeshComponent.SetAnimInstanceClass` (`self.SK_Body`) _st_npc_animclass)
  ;[1 1 1] Sets the MaxWalkSpeed / Subtracts a random value between 0 and 50 vor more variation
  (set `FloatingPawnMovement.MaxSpeed` (- (`KismetMathLibrary.Conv_IntToDouble` (`self.WalkSpeed_Max`)) (`KismetMathLibrary.RandomFloatInRange` 0.0 50.0)) (`self.FloatingPawnMovement`)))

(fn `UserConstructionScript`)