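; AI controller for NPCs that runs the BT_NPC behavior tree on BeginPlay.
; StartMoving stores the spawner and destination references and writes the destination to the Blackboard.
; BT_Change_Walk_Direction updates the Walk_Forward Blackboard key only when the value differs.
; An unconnected snippet would randomly pick one of two default navigation filter classes, but it never runs.
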(event `self.ReceiveBeginPlay`
  ;[1 1 1] Run Behaviour Tree
  (`self.RunBehaviorTree` "/Game/Blueprints/NPC/Behavior/BT_NPC.BT_NPC"))

(event `StartMoving`
  (params (Spawner :type "/Game/Blueprints/NPC/BP_Spawner Object Reference") (Destination :type "/Game/Blueprints/BP_MainTree Object Reference"))
  ;[1 1 1] Set SpawnerRef and DestinationRef / Also Sets Destination BlackboardValue
  (set `self.Spawner` Spawner)
  (set `self.Destination` Destination)
  (`BlackboardComponent.SetValueAsObject` (`self.Blackboard`) "Destination" Destination))

(event `BT_Change_Walk_Direction`
  (params (Forward :type Boolean))
  ;[1 1 1] Sets WalkDirection BlackboardValue
  (if (!= Forward (`BlackboardComponent.GetValueAsBool` (`self.Blackboard`) "Walk_Forward"))
    (`BlackboardComponent.SetValueAsBool` (`self.Blackboard`) "Walk_Forward" Forward)))

(fn `UserConstructionScript`)