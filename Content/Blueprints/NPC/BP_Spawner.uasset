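; Wave spawner that alternates a skippable build-phase countdown with enemy waves, growing the main tree before each wave.
; Wave tables supply enemy types and amounts; a chained timer spawns randomly picked NPCs, configured from DT_NPCs and sent toward the tree.
; Spawn points fall in a randomized band around world origin that widens after each wave spawns.
; Enemy removal dispatchers count deaths to end waves; clearing the last prints a win message.
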(event `self.ReceiveBeginPlay`
  (bind _returnvalue (`GameplayStatics.GetActorOfClass` "/Game/Blueprints/BP_MainTree.BP_MainTree_C"))
  (set `self.MainTree_Ref` _returnvalue)
  (`self.Set_TotalWave`)
  (`KismetSystemLibrary.Delay` 2.0))

(event `Set_TotalWave`
  ;[1 1 1] Set the total amount of waves for this level
  (bind _returnvalue (`DataTableFunctionLibrary.GetDataTableColumnAsString` (`self.DT_Waves`) "Enemy_Types"))
  (set `self.Wave_Total` (`KismetArrayLibrary.Array_Length` _returnvalue)))

(event `EnemyRemoved`
  ;[1 1 1] If a EnemyPawn calls the EnemyRemovedDispatcher this Function gets triggerd
  (`/Engine/EditorBlueprintResources/StandardMacros.IncrementInt` (`self.Enemies_Dead`)
    (:`  `
      (if (not (< (`self.Enemies_Dead`) (`self.Enemies_Total`)))
        (`self.Change_GamePhase`)))))

(event `Change_SpawnRadius`
  ;[1 1 1] Increase the radius where the enemies can´t spawn
  (`/Engine/EditorBlueprintResources/StandardMacros.IncrementInt` (`self.SpawnRadius`)))

(event `Spawn_NextWave`
  ;[1 1 1] -Count the Amount of enemies to spawn
  ; -reset the variables to default values
  ; -start the timer to spawn enemies
  (set `self.InWave` true)
  (bind _enemiestospawn (`self.CountEnemiesToSpawn`))
  (set `self.Enemies_Total` _enemiestospawn)
  (set `self.Enemies_Current` 0)
  (set `self.Enemies_Dead` 0)
  (set `self.SaveTime_Current` (`self.SaveTime_Max`))
  (set `self.Skip` false)
  (`self.Start_TimerSpawn`))

(event `Start_TimerBuildPhase`
  ;[1 1 1] A Timer for the build phase - reduce an int - SaveTimer == 0 starts the next wave
  ; if the player press the skip button -> the timer ends and starts the next wave
  (`KismetSystemLibrary.K2_SetTimerDelegate` (delegate `Reduce_SaveTime`) 1.0))

(event `Change_GamePhase`
  (bind _wave_current (`self.Wave_Current`))
  ;[1 1 1] Change the current game phase -
  (`self.ED_ChangePhase`)
  (if (`self.InWave`)
    (set `self.InWave` false)
    (`/Engine/EditorBlueprintResources/StandardMacros.IncrementInt` _wave_current
      (:`  `
        (if (> _wave_current (`self.Wave_Total`))
          (`KismetSystemLibrary.PrintString` "Won!!!" true true (struct :`R` 1.0 :`A` 1.0) 20.0)
          (else
            (`self.Start_TimerBuildPhase`)))))
    (else
      (`/Game/Blueprints/BP_MainTree.Grow` (`self.MainTree_Ref`))
      (`self.Spawn_NextWave`))))

(event `Reduce_SaveTime`
  (bind _savetime_current (`self.SaveTime_Current`))
  ;[1 1 1] A Timer for the build phase - reduce an int - SaveTimer == 0 starts the next wave
  ; if the player press the skip button -> the timer ends and starts the next wave
  (`/Engine/EditorBlueprintResources/StandardMacros.DecrementInt` _savetime_current
    (:`  `
      (if (> _savetime_current 0)
        (if (`self.Skip`)
          (`self.Change_GamePhase` :!label _label)
          (else
            (`self.Start_TimerBuildPhase`)))
        (else
          (goto _label))))))

(event `Start_TimerSpawn`
  ;[1 1 1] Starts SpawnTimer / Executes TimerSpawn in Intervals
  (`KismetSystemLibrary.K2_SetTimerDelegate` (delegate `TimerSpawn`) 0.1))

(event `TimerSpawn`
  ;[1 1 1] Starts SpawnTimer / Executes TimerSpawn in Intervals
  (bind _returnvalue (`self.Get_RandomEnemyToSpawn`))
  (`self.Spawn_SingleNPC` _returnvalue)
  (`/Engine/EditorBlueprintResources/StandardMacros.IncrementInt` (`self.Enemies_Current`)
    (:`  `
      (if (> (`self.Enemies_Total`) (`self.Enemies_Current`))
        (`self.Start_TimerSpawn`)
        (else
          (`self.Change_SpawnRadius`))))))

(event `Spawn_SingleNPC`
  (params (RowName :type Name))
  (bind (_returnvalue_location _returnvalue_rotation) (`KismetMathLibrary.BreakTransform` (`self.Get_SpawnTransform`)))
  ;[1 1 1] Spawn Enemy / Sets Variables by DataTable (DT_NPCS)
  (bind _returnvalue (`|GetDataTableRow` "/Game/Blueprints/Structs_Tables/DT_NPCs.DT_NPCs" RowName)
    (:`then`
      (bind _returnvalue_2 (`AIBlueprintHelperLibrary.SpawnAIFromClass` "/Game/Blueprints/NPC/CH_NPC.CH_NPC_C" "/Game/Blueprints/NPC/Behavior/BT_NPC.BT_NPC" _returnvalue_location _returnvalue_rotation true self))
      (bind _asch_npc (cast `/Game/Blueprints/NPC/CH_NPC` _returnvalue_2))
      (`/Game/Blueprints/NPC/CH_NPC.Set_Variables` _asch_npc _returnvalue)
      ;;[1 1 1 1 12] Bind EnemyRemoved to EnemyRemovedDispatcher of the spawned EnemyPawn
      (add `/Game/Blueprints/NPC/CH_NPC.RemoveEnemy` _asch_npc (`|CreateDelegate` :!event `EnemyRemoved`))
      (bind _asc_npc (cast `/Game/Blueprints/NPC/C_NPC` (`AIBlueprintHelperLibrary.GetAIController` _asch_npc)))
      (`/Game/Blueprints/NPC/C_NPC.StartMoving` _asc_npc self (`self.MainTree_Ref`)))))

(fn `CountEnemiesToSpawn`
  (returns (EnemiesToSpawn :type Integer))
  (locals (Counter :type Integer))
  (`KismetArrayLibrary.Array_Clear` (`self.Enemies_AmountSpawned`))
  (bind _returnvalue (`|GetDataTableRow` (`self.DT_Waves`) (`KismetStringLibrary.Conv_StringToName` (`KismetStringLibrary.Conv_IntToString` (`self.Wave_Current`))))
    (:`then`
      (bind (_enemy_types _enemy_amount) (break `/Game/Blueprints/Structs_Tables/ST_Waves` _returnvalue))
      (for (_array_element _array_index) _enemy_amount
        (set `local.Counter` (+ _array_element (`local.Counter`)))
        (`KismetArrayLibrary.Array_Set` (`self.Enemies_AmountSpawned`) _array_index 0 true))
      (set `self.Enemies_Types` _enemy_types)
      (set `self.Enemies_Amount` _enemy_amount)
      (return (`local.Counter`)))))

(fn `Get_RandomEnemyToSpawn`
  (returns (ReturnValue :type Name))
  (locals (Local_Index :type Integer :default 0))
  (set `local.Local_Index` (`.OutIndex` (`KismetArrayLibrary.Array_Random` (`self.Enemies_Types`))))
  (`KismetArrayLibrary.Array_Set` (`self.Enemies_AmountSpawned`) (`local.Local_Index`) (+ (`|GetArrayItem` (`self.Enemies_AmountSpawned`) (`local.Local_Index`)) 1) true)
  (if (not (> (`|GetArrayItem` (`self.Enemies_Amount`) (`local.Local_Index`)) (`|GetArrayItem` (`self.Enemies_AmountSpawned`) (`local.Local_Index`))))
    (`KismetArrayLibrary.Array_Remove` (`self.Enemies_TypesSpawned`) (`local.Local_Index`))
    (`KismetArrayLibrary.Array_Remove` (`self.Enemies_AmountSpawned`) (`local.Local_Index`)))
  (return (`KismetStringLibrary.Conv_StringToName` (`|GetEnumeratorNameAsString` (`|GetArrayItem` (`self.Enemies_Types`) (`local.Local_Index`))))))

(fn `Get_SpawnDistance`
  (returns (SpawnPoint :type "Vector Structure"))
  (locals (Local_Bound :type Integer :default 0) (Local_UnBound :type Integer :default 0))
  (bind _returnvalue (* (`self.SpawnRadius`) (`self.Grow`)))
  (bind _returnvalue_2 (* _returnvalue 2))
  (bind _returnvalue_3 (`KismetMathLibrary.RandomIntegerInRange` _returnvalue (+ _returnvalue (`KismetMathLibrary.RandomIntegerInRange` 0 _returnvalue_2))))
  (set `local.Local_Bound` (`KismetMathLibrary.SelectInt` _returnvalue_3 (* _returnvalue_3 -1) (`KismetMathLibrary.RandomBool`)))
  (set `local.Local_UnBound` (`KismetMathLibrary.RandomIntegerInRange` (* _returnvalue_2 -1) _returnvalue_2))
  (if (`KismetMathLibrary.RandomBool`)
    (return (`KismetMathLibrary.MakeVector` (`KismetMathLibrary.Conv_IntToDouble` (`local.Local_Bound`)) (`KismetMathLibrary.Conv_IntToDouble` (`local.Local_UnBound`))))
    (else
      (return (`KismetMathLibrary.MakeVector` (`KismetMathLibrary.Conv_IntToDouble` (`local.Local_UnBound`)) (`KismetMathLibrary.Conv_IntToDouble` (`local.Local_Bound`)))))))

(fn `Get_SpawnTransform`
  (returns (ReturnValue :type "Transform Structure"))
  (return (`KismetMathLibrary.MakeTransform` (`self.Get_SpawnDistance`))))

(fn `UserConstructionScript`)