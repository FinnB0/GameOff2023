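; Foliage spawner actor that grows scattered static meshes around the main tree, in a band that moves with each spawn.
; On BeginPlay it finds BP_MainTree and binds to its grow dispatcher.
; SpawnGrass adds mesh components at random angles and distances from its own location at zero scale, then shifts the offset range.
; A timeline scales each new batch up to random sizes, then clears the batch arrays.
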(event `self.ReceiveBeginPlay`
  ;[1 1 1] Get the MainTree as a Reference on Begin Play
  (`self.GetMainTreeRef`))

(event `SpawnGrass`
  ;[1 1 1] Spawns the Instances of Foliage around the MainTree
  (for _ (range (+ (`self.Foliage Amount`) 1))
    (bind _returnvalue (`AddComponent|NODE_AddStaticMeshComponent-0` :`RelativeTransform` (`KismetMathLibrary.MakeTransform` (+ (`self.K2_GetActorLocation`) (* (`KismetMathLibrary.GetForwardVector` (`KismetMathLibrary.MakeRotator` 0.0 0.0 (`KismetMathLibrary.RandomFloatInRange` 0.0 360.0))) (+ (`self.StartDistance`) (`KismetMathLibrary.RandomFloatInRange` (`self.MinOffset`) (`self.MaxOffset`))))) (`KismetMathLibrary.MakeRotator` 0.0 0.0 (`KismetMathLibrary.RandomFloatInRange` 0.0 360.0)) (0.0 0.0 0.0))))
    (`KismetArrayLibrary.Array_Add` (`self.NewFoliageMeshes`) _returnvalue)
    (`KismetArrayLibrary.Array_Add` (`self.NewFoliageScale`) (`KismetMathLibrary.RandomFloatInRange` 0.5 2.0)))
  (set `self.MaxOffset` (+ (`self.MaxOffset`) (`self.MaxOffsetAddition`)))
  (set `self.MinOffset` (+ (`self.MinOffset`) (`self.MinOffsetAddition`)))
  (`TimelineComponent.PlayFromStart` (`self.GrowTimer`)))

(fn `GetMainTreeRef`
  (bind _returnvalue (`GameplayStatics.GetActorOfClass` "/Game/Blueprints/BP_MainTree.BP_MainTree_C"))
  (bind _output_get (set `self.BP_MainTree` _returnvalue))
  (add `/Game/Blueprints/BP_MainTree.GrowDispatcher` _output_get (`|CreateDelegate` :!event `SpawnGrass`)))

(fn `UserConstructionScript`)