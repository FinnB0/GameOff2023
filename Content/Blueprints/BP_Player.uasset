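; BP_Player is a player camera rig with spring-arm zoom and yaw rotation through Enhanced Input.
; The construction script applies camera angle, distance and height; zoom input reuses the clamped distance setter.
; Rotate input turns controller yaw and hides the cursor via ToggleInteraction until completed.
; Forward and right movement offset nodes exist but are disconnected, so the file performs no movement.
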(event `self.ReceiveBeginPlay`
  (message `EnhancedInputSubsystemInterface.AddMappingContext` (pcsubsystem `EnhancedInputLocalPlayerSubsystem` (`GameplayStatics.GetPlayerController` 0)) "/Game/Input/IMC_Default.IMC_Default" 0 (struct)))

(event `EnhancedInput|/Game/Input/IA_MoveForward`
  (params (ActionValue :type "Float (double-precision)") (ElapsedSeconds :type "Float (double-precision)") (TriggeredSeconds :type "Float (double-precision)") (InputAction :type "InputAction Object Reference" :default "/Game/Input/IA_MoveForward.IA_MoveForward"))
  ;[1 1 1] Movement
)

(event `EnhancedInput|/Game/Input/IA_MoveRight`
  (params (ActionValue :type "Float (double-precision)") (ElapsedSeconds :type "Float (double-precision)") (TriggeredSeconds :type "Float (double-precision)") (InputAction :type "InputAction Object Reference" :default "/Game/Input/IA_MoveRight.IA_MoveRight"))
  ;[1 1 1] Movement
)

(event `EnhancedInput|/Game/Input/IA_Zoom`
  (params (ActionValue :type "Float (double-precision)") (ElapsedSeconds :type "Float (double-precision)") (TriggeredSeconds :type "Float (double-precision)") (InputAction :type "InputAction Object Reference" :default "/Game/Input/IA_Zoom.IA_Zoom"))
  ;[1 1 1] Movement
  (:`Triggered`
    (`self.SetCameraDistance` (+ (`self.CameraDistance`) (* ActionValue (`self.ZoomSpeed`))))))

(event `EnhancedInput|/Game/Input/IA_Rotate`
  (params (ActionValue :type Boolean) (ElapsedSeconds :type "Float (double-precision)") (TriggeredSeconds :type "Float (double-precision)") (InputAction :type "InputAction Object Reference" :default "/Game/Input/IA_Rotate.IA_Rotate"))
  (bind _returnvalue (`self.GetController`))
  (bind (_returnvalue_roll _returnvalue_pitch _returnvalue_yaw) (`KismetMathLibrary.BreakRotator` (`Controller.GetControlRotation` _returnvalue)))
  ;[1 1 1] Movement
  (:`Triggered`
    (`Controller.SetControlRotation` _returnvalue (`KismetMathLibrary.MakeRotator` _returnvalue_roll _returnvalue_pitch (+ _returnvalue_yaw (* (`self.GetInputAxisKeyValue`) (`self.RotationSpeed`)))))
    (`self.ToggleInteraction` false))
  (:`Completed`
    (`self.ToggleInteraction` true)))

(fn `SetCameraAngle`
  (params (CameraAngle :type "Float (double-precision)"))
  (bind _springarm (`self.SpringArm`))
  (bind (_relativerotation_roll _relativerotation_pitch _relativerotation_yaw) (`KismetMathLibrary.BreakRotator` (`SceneComponent.RelativeRotation` _springarm)))
  (`SceneComponent.K2_SetRelativeRotation` _springarm (`KismetMathLibrary.MakeRotator` _relativerotation_roll (* CameraAngle -1.0) _relativerotation_yaw) false false))

(fn `SetCameraDistance`
  (params (CameraDistance :type "Float (double-precision)"))
  (bind _output_get (set `self.CameraDistance` (`KismetMathLibrary.FClamp` CameraDistance (`self.CameraDistanceMin`) (`self.CameraDistanceMax`))))
  (set `SpringArmComponent.TargetArmLength` _output_get (`self.SpringArm`)))

(fn `SetCameraHeight`
  (`SceneComponent.K2_SetRelativeLocation` (`self.SpringArm`) (`KismetMathLibrary.MakeVector` 0.0 0.0 (`self.CameraHeight`)) false false))

(fn `ToggleInteraction`
  (params (bCanInteract :type Boolean))
  (bind _output_get (set `self.bCanInteract` bCanInteract))
  (if _output_get
    (set `PlayerController.bShowMouseCursor` true (`GameplayStatics.GetPlayerController` 0))
    (else
      (set `PlayerController.bShowMouseCursor` false (`GameplayStatics.GetPlayerController` 0)))))

(fn `UserConstructionScript`
  (`self.SetCameraAngle` (`self.CameraAngle`))
  (`self.SetCameraDistance` (`self.CameraDistance`))
  (`self.SetCameraHeight`))