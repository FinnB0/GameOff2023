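; Player pawn with an orbit-style camera that places towers on the main tree's "SecondRoot" components.
; Enhanced Input drives controller yaw rotation, forward distance and scaled zoom through two clamped spring arms.
; Each tick a cursor trace moves a ghost, yawed relative to the tree, and colors it by placement validity; interacting spawns and attaches BP_Tower at its transform.
; Debug-style keys call the game mode to randomize MetaSound or switch game state.
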(event `Key|Tab`
  (params (Key :type "Key Structure"))
  ;[1 1 1] Switch GameState to Build/Combat-Mode
  (:`Pressed`
    (`/Game/Blueprints/Game/GMB_Game.RandomizeMetaSound` (cast `/Game/Blueprints/Game/GMB_Game` (`GameplayStatics.GetGameMode`) :!pure true))))

(event `self.ReceiveBeginPlay`
  (message `EnhancedInputSubsystemInterface.AddMappingContext` (pcsubsystem `EnhancedInputLocalPlayerSubsystem` (`GameplayStatics.GetPlayerController` 0)) "/Game/Input/IMC_Default.IMC_Default" 0 (struct))
  (`self.CreateMainTreeReference`)
  (`self.CreateInteractionGhost`))

(event `self.ReceiveTick`
  (params (DeltaSeconds :type "Float (single-precision)"))
  (`self.Set Interaction GhostTransform`))

(event `Key|P`
  (params (Key :type "Key Structure"))
  ;[1 1 1] Switch GameState to Paused
  (:`Pressed`
    (`/Game/Blueprints/Game/GMB_Game.SwitchGameState` (cast `/Game/Blueprints/Game/GMB_Game` (`GameplayStatics.GetGameMode`) :!pure true) "NewEnumerator0")))

(event `EnhancedInput|/Game/Input/IA_MoveForward`
  (params (ActionValue :type "Float (double-precision)") (ElapsedSeconds :type "Float (double-precision)") (TriggeredSeconds :type "Float (double-precision)") (InputAction :type "InputAction Object Reference" :default "/Game/Input/IA_MoveForward.IA_MoveForward"))
  ;[1 1 1] Input
  ;;[1 1 1] Moving
  (:`Triggered`
    (`self.MoveForward` ActionValue)))

(event `MoveForward`
  (params (ActionValue :type "Float (double-precision)") (bIsMouseInput :type Boolean))
  ;[1 1 1] Input
  ;;[1 1 1] Moving
  (`self.SetCameraDistance` (+ (`self.CameraDistance`) (* (`KismetMathLibrary.SelectFloat` (`self.GetInputAxisKeyValue`) ActionValue bIsMouseInput) (`self.MoveSpeed`)))))

(event `EnhancedInput|/Game/Input/IA_MouseRotate`
  (params (ActionValue :type "Float (double-precision)") (ElapsedSeconds :type "Float (double-precision)") (TriggeredSeconds :type "Float (double-precision)") (InputAction :type "InputAction Object Reference" :default "/Game/Input/IA_MouseRotate.IA_MouseRotate"))
  ;[1 1 1] Input
  ;;[1 1 1] Rotate and Move with Mouse
  (:`Triggered`
    (`self.Rotate` 0.0 true)
    (`self.MoveForward` 0.0 true)))

(event `EnhancedInput|/Game/Input/IA_Rotate`
  (params (ActionValue :type "Float (double-precision)") (ElapsedSeconds :type "Float (double-precision)") (TriggeredSeconds :type "Float (double-precision)") (InputAction :type "InputAction Object Reference" :default "/Game/Input/IA_Rotate.IA_Rotate"))
  ;[1 1 1] Input
  ;;[1 1 1] Rotate
  (:`Triggered`
    (`self.Rotate` ActionValue)))

(event `Rotate`
  (params (ActionValue :type "Float (double-precision)") (bIsMouseInput :type Boolean))
  (bind _returnvalue (`self.GetController`))
  (bind (_returnvalue_roll _returnvalue_pitch _returnvalue_yaw) (`KismetMathLibrary.BreakRotator` (`Controller.GetControlRotation` _returnvalue)))
  ;[1 1 1] Input
  ;;[1 1 1] Rotate
  (`Controller.SetControlRotation` _returnvalue (`KismetMathLibrary.MakeRotator` _returnvalue_roll _returnvalue_pitch (+ _returnvalue_yaw (* (`KismetMathLibrary.SelectFloat` (`self.GetInputAxisKeyValue`) ActionValue bIsMouseInput) (`self.RotationSpeed`))))))

(event `EnhancedInput|/Game/Input/IA_Interact`
  (params (ActionValue :type Boolean) (ElapsedSeconds :type "Float (double-precision)") (TriggeredSeconds :type "Float (double-precision)") (InputAction :type "InputAction Object Reference" :default "/Game/Input/IA_Interact.IA_Interact"))
  (bind (_bblockinghit _binitialoverlap _time _distance _location _impactpoint _normal _impactnormal _physmat _hitactor _hitcomponent) (`GameplayStatics.BreakHitResult` (`PlayerController.GetHitResultUnderCursorForObjects` (`GameplayStatics.GetPlayerController` 0) (`|MakeArray` "ObjectTypeQuery1" "ObjectTypeQuery2" :!type "EObjectTypeQuery Enum") true)))
  ;[1 1 1] Input
  ;;[1 1 1] Interact
  (:`Started`
    (if (`self.bCanInteract`)
      (if _bblockinghit
        (if (`KismetStringLibrary.Contains` (`KismetSystemLibrary.GetDisplayName` _hitcomponent) "SecondRoot")
          (bind _returnvalue (`|SpawnActorFromClass` "/Game/Blueprints/BP_Tower.BP_Tower_C" (`self.GetTransform` (`self.BP_InteractionGhost`)) "Undefined" "MultiplyWithRoot" null null))
          (`self.K2_AttachToActor` _returnvalue _hitactor "None" "KeepWorld" "KeepWorld" "KeepWorld" true))))))

(event `EnhancedInput|/Game/Input/IA_Zoom`
  (params (ActionValue :type "Float (double-precision)") (ElapsedSeconds :type "Float (double-precision)") (TriggeredSeconds :type "Float (double-precision)") (InputAction :type "InputAction Object Reference" :default "/Game/Input/IA_Zoom.IA_Zoom"))
  ;[1 1 1] Input
  ;;[1 1 1] Zoom
  (:`Triggered`
    (`self.SetCameraZoomDistance` (+ (`self.CameraZoomDistance`) (* ActionValue (`self.ZoomSpeed`) (`KismetMathLibrary.FClamp` (/ (`self.CameraZoomDistance`) (`self.CameraZoomDistanceMax`)) 0.5))))))

(event `EnhancedInput|/Game/Input/IA_Quit`
  (params (ActionValue :type Boolean) (ElapsedSeconds :type "Float (double-precision)") (TriggeredSeconds :type "Float (double-precision)") (InputAction :type "InputAction Object Reference" :default "/Game/Input/IA_Quit.IA_Quit"))
  ;[1 1 1] Input
  ;;[1 1 1] Quit Game
  (:`Started`
    (`KismetSystemLibrary.QuitGame` null "Quit")))

(fn `CreateInteractionGhost`
  ;[1 1 1] Creates the InteractionGhost
  (bind _returnvalue (`|SpawnActorFromClass` "/Game/Blueprints/Player/BP_InteractionGhost.BP_InteractionGhost_C" (`KismetMathLibrary.MakeTransform` (0.0 0.0 0.0)) "Undefined" "MultiplyWithRoot" null null))
  (set `self.BP_InteractionGhost` _returnvalue))

(fn `CreateMainTreeReference`
  (bind _returnvalue (`GameplayStatics.GetActorOfClass` "/Game/Blueprints/BP_MainTree.BP_MainTree_C"))
  (set `self.BP_MainTree` _returnvalue))

(fn `Set Interaction GhostTransform`
  (bind _bp_interactionghost (`self.BP_InteractionGhost`))
  (bind (_bblockinghit _binitialoverlap _time _distance _location _impactpoint _normal _impactnormal _physmat _hitactor _hitcomponent) (`GameplayStatics.BreakHitResult` (`PlayerController.GetHitResultUnderCursorForObjects` (`GameplayStatics.GetPlayerController` 0) (`|MakeArray` "ObjectTypeQuery1" "ObjectTypeQuery2" :!type "EObjectTypeQuery Enum") true)))
  (bind (_returnvalue_roll _returnvalue_pitch _returnvalue_yaw) (`KismetMathLibrary.BreakRotator` (`KismetMathLibrary.MakeRotFromZ` (- _location (`self.K2_GetActorLocation` (`self.BP_MainTree`))))))
  (`/Engine/EditorBlueprintResources/StandardMacros.IsValid` (`self.BP_InteractionGhost`)
    (:`Is Valid`
      (if _bblockinghit
        (`self.K2_SetActorLocationAndRotation` (`self.BP_InteractionGhost`) _location (`KismetMathLibrary.MakeRotator` 0.0 0.0 _returnvalue_yaw) false false)
        (if (`KismetStringLibrary.Contains` (`KismetSystemLibrary.GetDisplayName` _hitcomponent) "SecondRoot")
          (`/Game/Blueprints/Player/BP_InteractionGhost.ToggleColor` _bp_interactionghost true)
          (else
            (`/Game/Blueprints/Player/BP_InteractionGhost.ToggleColor` _bp_interactionghost false)))))))

(fn `SetCameraAngle`
  (params (CameraAngle :type "Float (double-precision)"))
  (bind _distancezoom (`self.DistanceZoom`))
  (bind (_relativerotation_roll _relativerotation_pitch _relativerotation_yaw) (`KismetMathLibrary.BreakRotator` (`SceneComponent.RelativeRotation` _distancezoom)))
  (`SceneComponent.K2_SetRelativeRotation` _distancezoom (`KismetMathLibrary.MakeRotator` _relativerotation_roll (* CameraAngle -1.0) _relativerotation_yaw) false false))

(fn `SetCameraDistance`
  (params (CameraDistance :type "Float (double-precision)"))
  ;[1 1 1] Sets the Distance Between the Player and the MainTree
  (bind _output_get (set `self.CameraDistance` (`KismetMathLibrary.FClamp` CameraDistance (`self.CameraDistanceMin`) (`self.CameraDistanceMax`))))
  (set `SpringArmComponent.TargetArmLength` _output_get (`self.DistanceForward`)))

(fn `SetCameraHeight`
  (`SceneComponent.K2_SetRelativeLocation` (`self.DefaultSceneRoot`) (`KismetMathLibrary.MakeVector` 0.0 0.0 (`self.CameraHeight`)) false false))

(fn `SetCameraZoomDistance`
  (params (CameraDistance :type "Float (double-precision)"))
  (bind _output_get (set `self.CameraZoomDistance` (`KismetMathLibrary.FClamp` CameraDistance (`self.CameraZoomDistanceMin`) (`self.CameraZoomDistanceMax`))))
  (set `SpringArmComponent.TargetArmLength` _output_get (`self.DistanceZoom`)))

(fn `ToggleInteraction`
  (params (bCanInteract :type Boolean))
  (bind _output_get (set `self.bCanInteract` bCanInteract))
  (if _output_get
    (`self.SetActorHiddenInGame` (`self.BP_InteractionGhost`) false)
    (else
      (`self.SetActorHiddenInGame` (`self.BP_InteractionGhost`) true))))

(fn `UserConstructionScript`
  (`self.SetCameraAngle` (`self.CameraAngle`))
  (`self.SetCameraZoomDistance` (`self.CameraZoomDistance`))
  (`self.SetCameraHeight`))