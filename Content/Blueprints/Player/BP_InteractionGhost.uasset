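; BP_InteractionGhost is the player's interaction preview actor, showing a ghost mesh and an attack-radius decal.
; On BeginPlay it creates dynamic material instances for both components.
; ToggleColor tints both by Select, Build or Recycle mode, switching to a no-interaction color when interaction is unavailable.
; SetRadius scales the decal, and Tick keeps it under the actor at world Z zero.
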(event `self.ReceiveBeginPlay`
  ;[1 1 1] Create Material Intstancies
  (`self.CreateMaterialInstancies`))

(event `ToggleColor`
  (params (bCanInteract :type Boolean) (InteractionMode :type "/Game/Blueprints/Enums/E_InteractionMode Enum" :default "NewEnumerator0"))
  (bind _colornointeraction (`self.ColorNoInteraction`))
  (bind _returnvalue (`KismetMathLibrary.SelectColor` (select `/Game/Blueprints/Enums/E_InteractionMode` InteractionMode :`NewEnumerator0` (`self.ColorSelect`) :`NewEnumerator1` (`self.ColorBuild`) :`NewEnumerator2` (`self.ColorRecycle`)) (select `/Game/Blueprints/Enums/E_InteractionMode` InteractionMode :`NewEnumerator0` _colornointeraction :`NewEnumerator1` _colornointeraction :`NewEnumerator2` _colornointeraction) bCanInteract))
  ;[1 1 1] Toggles the Color of the Decale and the Mesh
  (`MaterialInstanceDynamic.SetVectorParameterValue` (`self.MeshMI`) "PulseColor" _returnvalue)
  (`MaterialInstanceDynamic.SetVectorParameterValue` (`self.DecaleMI`) "EmissiveColor" _returnvalue))

(event `SetRadius`
  (params (Radius :type "Float (double-precision)"))
  ;[1 1 1] Sets Decales Radius
  (`SceneComponent.SetWorldScale3D` (`self.AttackRadiusDecal`) (`KismetMathLibrary.MakeVector` 1.0 Radius Radius)))

(event `self.ReceiveTick`
  (params (DeltaSeconds :type "Float (single-precision)"))
  ;[1 1 1] Sets Decale to the Ground  (Zeros Z)
  (`self.SetDecaleLocation`))

(fn `CreateMaterialInstancies`
  (bind _ghostmesh (`self.GhostMesh`))
  (bind _returnvalue (`PrimitiveComponent.CreateDynamicMaterialInstance` _ghostmesh 0 (`PrimitiveComponent.GetMaterial` _ghostmesh 0) "None"))
  (set `self.MeshMI` _returnvalue)
  (bind _returnvalue_2 (`DecalComponent.CreateDynamicMaterialInstance` (`self.AttackRadiusDecal`)))
  (set `self.DecaleMI` _returnvalue_2))

(fn `SetDecaleLocation`
  (bind (_returnvalue_x _returnvalue_y) (`KismetMathLibrary.BreakVector` (`self.K2_GetActorLocation`)))
  (`SceneComponent.K2_SetWorldLocation` (`self.AttackRadiusDecal`) (`KismetMathLibrary.MakeVector` _returnvalue_x _returnvalue_y) false false))

(fn `UserConstructionScript`)